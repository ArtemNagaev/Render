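; Test Blueprint that evaluates a piecewise math function, CalculateC, and shows the result on screen.
; BeginPlay calls it with fixed inputs and prints the returned value.
; CalculateC branches on A and B to return the square root of the product of their absolute values, their sum, or the cube root of their sum.
; Tick and the construction script are empty.
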(event `self.ReceiveBeginPlay`
  (bind _returnc (`self.CalculateC` 15.0 11.0))
  (`KismetSystemLibrary.PrintString` (`KismetStringLibrary.Conv_DoubleToString` _returnc) true false (struct :`G` 0.66 :`B` 1.0 :`A` 1.0) 10.0))

(event `self.ReceiveTick`
  (params (DeltaSeconds :type "Float (single-precision)")))

(fn `CalculateC`
  (params (A :type "Float (double-precision)") (B :type "Float (double-precision)"))
  (returns (ReturnC :type "Float (double-precision)"))
  (locals (c_local :type "Float (double-precision)") (a_local :type "Float (double-precision)") (b_local :type "Float (double-precision)"))
  (set `local.a_local` A)
  (set `local.b_local` B)
  (if (and (!= (`local.a_local`) 15.0) (> (`local.b_local`) 10.0))
    (bind _output_get (set `local.c_local` (`KismetMathLibrary.Sqrt` (* (`KismetMathLibrary.Abs` (`local.a_local`)) (`KismetMathLibrary.Abs` (`local.b_local`))))))
    (return _output_get)
    (elif (>= (`local.a_local`) 15.0)
      (bind _output_get_2 (set `local.c_local` (+ (`local.a_local`) (`local.b_local`))))
      (return _output_get_2)
      (else
        (bind _output_get_3 (set `local.c_local` (`KismetMathLibrary.MultiplyMultiply_FloatFloat` (+ (`local.a_local`) (`local.b_local`)) (/ 1.0 3.0))))
        (return _output_get_3)))))

(fn `UserConstructionScript`)