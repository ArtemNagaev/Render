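; TestCase8 is a functional test Blueprint that checks the CalculateC function on a GameMode.
; On StartTest it calls CalculateC with fixed inputs and compares the result to the expected sum of those inputs within a tight float tolerance.
; It then finishes the test as succeeded or failed with an empty message.
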(event `self.ReceiveStartTest`
  (`parent.ReceiveStartTest`)
  (bind _returnc (`/Game/Blueprints/Function.CalculateC` (`self.GameMode`) 15.0 9.0))
  (if (`KismetMathLibrary.NearlyEqual_FloatFloat` _returnc 24.0)
    (`self.FinishTest` "Succeeded")
    (else
      (`self.FinishTest` "Failed"))))

(fn `UserConstructionScript`
  (`parent.UserConstructionScript`))